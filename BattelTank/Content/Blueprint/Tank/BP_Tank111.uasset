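; Player-controlled tank Blueprint that handles camera aiming, track throttle and firing input.
; On BeginPlay it registers the barrel and turret through setter functions defined outside its graphs.
; Aim axes rotate an azimuth gimbal in yaw and a spring arm in pitch, scaled by frame delta time.
; Left and right throttle axes pass straight to SetTrottele, and the Fire action calls Fire.
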(event `self.ReceiveBeginPlay`
  (`self.SetBarrelReference` (`self.TankBarrel`))
  (`self.SetTurretlReference` (`self.TankTurret`)))

(event `InputAxis|AimAzimuth`
  (params (AxisValue :type "Float (single-precision)"))
  (`SceneComponent.K2_AddLocalRotation` (`self.azimuth gimbal`) (`KismetMathLibrary.MakeRotator` 0.0 0.0 (* AxisValue (`GameplayStatics.GetWorldDeltaSeconds`) 100.0)) false false))

(event `InputAxis|LeftTrackThrottle`
  (params (AxisValue :type "Float (single-precision)"))
  (`TankTrack.SetTrottele` AxisValue))

(event `InputAxis|RighetTrackThrottle`
  (params (AxisValue :type "Float (single-precision)"))
  (`TankTrack.SetTrottele` AxisValue))

(event `InputAxis|AimElevation`
  (params (AxisValue :type "Float (single-precision)"))
  (`SceneComponent.K2_AddLocalRotation` (`self.SpringArm`) (`KismetMathLibrary.MakeRotator` 0.0 (* AxisValue (`GameplayStatics.GetWorldDeltaSeconds`) 100.0)) false false))

(event `InputAction|Fire`
  (params (Key :type "Key Structure"))
  (:`Pressed`
    (`self.Fire`)))

(fn `UserConstructionScript`)