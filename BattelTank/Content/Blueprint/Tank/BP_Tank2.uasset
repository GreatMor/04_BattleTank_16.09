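; BP_Tank2 is a player-controllable tank Blueprint that handles camera aiming, driving and firing input.
; On BeginPlay it hands the barrel and turret to TankAiming and both tracks to TankMovement.
; Aim axes rotate an azimuth gimbal and spring arm, scaled by delta time for frame-rate independence.
; Move and turn axes pass intent to TankMovement, and the Fire action calls Fire.
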(event `self.ReceiveBeginPlay`
  (`TankAimingComponent.Initilaize` (`self.TankAiming`) (`self.TankBarrel`) (`self.TankTurret`))
  (`TankMovementComponent.Initilaize` (`self.TankMovement`) (`self.LeftTrack`) (`self.RighetTrack`)))

(event `InputAxis|AimAzimuth`
  (params (AxisValue :type "Float (single-precision)"))
  ;[1 1 1] Aim setup
  (`SceneComponent.K2_AddLocalRotation` (`self.azimuth gimbal`) (`KismetMathLibrary.MakeRotator` 0.0 0.0 (* AxisValue (`GameplayStatics.GetWorldDeltaSeconds`) 100.0)) false false))

(event `InputAxis|AimElevation`
  (params (AxisValue :type "Float (single-precision)"))
  ;[1 1 1] Aim setup
  (`SceneComponent.K2_AddLocalRotation` (`self.SpringArm`) (`KismetMathLibrary.MakeRotator` 0.0 (* AxisValue (`GameplayStatics.GetWorldDeltaSeconds`) 100.0)) false false))

(event `InputAxis|MoveForward`
  (params (AxisValue :type "Float (single-precision)"))
  ;[1 1 1] Aim setup
  (`TankMovementComponent.IntendMoveForward` (`self.TankMovement`) AxisValue))

(event `InputAxis|Turn Righet And Left`
  (params (AxisValue :type "Float (single-precision)"))
  ;[1 1 1] Aim setup
  (`TankMovementComponent.IntendTurnRighet` (`self.TankMovement`) AxisValue))

(event `InputAction|Fire`
  (params (Key :type "Key Structure"))
  (:`Pressed`
    (`self.Fire`)))

(fn `UserConstructionScript`)